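; BP_Bullet is a projectile actor that flies along the world X axis and destroys itself after one second.
; Tick accumulates elapsed time in a Lifespan variable and, until that limit, offsets the bullet at four times BP_Player's ForwardSpeed, scaled by delta time.
; The player is looked up with GetActorOfClass on each moving tick, and the Blueprint has no hit or overlap logic.
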(event `self.ReceiveTick`
  (params (DeltaSeconds :type "Float (single-precision)"))
  (bind _output_get (set `self.Lifespan` (+ DeltaSeconds (`self.Lifespan`))))
  (if (>= _output_get 1.0)
    (`self.K2_DestroyActor`)
    (else
      (bind _returnvalue (`GameplayStatics.GetActorOfClass` "/Game/InfiniteMatrix/Blueprints/BP_Player.BP_Player_C"))
      (`self.K2_AddActorWorldOffset` (`KismetMathLibrary.MakeVector` (* DeltaSeconds (* (`/Game/InfiniteMatrix/Blueprints/BP_Player.ForwardSpeed` _returnvalue) 4.0)))))))

(fn `UserConstructionScript`)